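; Sword-wielding enemy character that detects the player and exposes whether the player is within combat range.
; Tagged overlaps on SearchRange and CombatRange set the found state, player reference and combat flag, while capsule overlaps forward to handler functions.
; Tick snaps the sword to its hand socket, briefly enables its collision during attacks and destroys the actor after a death delay.
; When IsStop is set, Tick instead pins the enemy at its last saved location.
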(event OnComponentBeginOverlap(CombatRange)
  (params (OverlappedComponent :type Primitive%20Component%20Object%20Reference) (OtherActor :type Actor%20Object%20Reference) (OtherComp :type Primitive%20Component%20Object%20Reference) (OtherBodyIndex :type Integer) (bFromSweep :type Boolean) (SweepResult :type Hit%20Result%20Structure%20%28by%20ref%29))
  (Utilities|IsValid OtherActor
    (:Is%20Valid
      (if (Components|ComponentHasTag OtherComp "Player")
        (Variables|Default|SetIsCombatRange true)))))

(event OnComponentBeginOverlap(CapsuleComponent)
  (params (OverlappedComponent :type Primitive%20Component%20Object%20Reference) (OtherActor :type Actor%20Object%20Reference) (OtherComp :type Primitive%20Component%20Object%20Reference) (OtherBodyIndex :type Integer) (bFromSweep :type Boolean) (SweepResult :type Hit%20Result%20Structure%20%28by%20ref%29))
  (Class|MyEnemy|OnBeginOverlap OverlappedComponent OtherActor OtherComp OtherBodyIndex bFromSweep))

(event OnComponentEndOverlap(CapsuleComponent)
  (params (OverlappedComponent :type Primitive%20Component%20Object%20Reference) (OtherActor :type Actor%20Object%20Reference) (OtherComp :type Primitive%20Component%20Object%20Reference) (OtherBodyIndex :type Integer))
  (Class|MyEnemy|OnEndOverlap OverlappedComponent OtherActor OtherComp OtherBodyIndex))

(event OnComponentEndOverlap(CombatRange)
  (params (OverlappedComponent :type Primitive%20Component%20Object%20Reference) (OtherActor :type Actor%20Object%20Reference) (OtherComp :type Primitive%20Component%20Object%20Reference) (OtherBodyIndex :type Integer))
  (if (Components|ComponentHasTag OtherComp "Player")
    (Variables|Default|SetIsCombatRange false)))

(event OnComponentBeginOverlap(SearchRange)
  (params (OverlappedComponent :type Primitive%20Component%20Object%20Reference) (OtherActor :type Actor%20Object%20Reference) (OtherComp :type Primitive%20Component%20Object%20Reference) (OtherBodyIndex :type Integer) (bFromSweep :type Boolean) (SweepResult :type Hit%20Result%20Structure%20%28by%20ref%29))
  (if (Components|ComponentHasTag OtherComp "Player")
    (Class|MyEnemy|SetisFound true)
    (Variables|Default|SetPlayer OtherActor)))

(event OnComponentEndOverlap(SearchRange)
  (params (OverlappedComponent :type Primitive%20Component%20Object%20Reference) (OtherActor :type Actor%20Object%20Reference) (OtherComp :type Primitive%20Component%20Object%20Reference) (OtherBodyIndex :type Integer))
  (if (Components|ComponentHasTag OtherComp "Player")
    (Class|MyEnemy|SetisFound false)))

(event EventTick
  (params (DeltaSeconds :type Float%20%28single-precision%29))
  (bind _mesh (Variables|Character|GetMesh))
  (if (Variables|Default|GetIsStop)
    (Transformation|SetActorLocation (Variables|Default|GetPauseLocation) false false)
    (else
      (Variables|Default|SetPauseLocation (Transformation|GetActorLocation))
      (Utilities|FlowControl|Sequence
        (:then_0
          (bind _returnvalue (Class|MyEnemy|GetIsDead))
          (if _returnvalue
            (Utilities|FlowControl|Delay 2.0)
            (Actor|DestroyActor)))
        (:then_1
          (if (Variables|Default|GetIsAttack)
            (Collision|SetCollisionEnabled (Variables|Default|GetSwordCollision) "QueryAndPhysics")
            (Utilities|FlowControl|Delay 0.3)
            (Variables|Default|SetIsAttack false)
            (else
              (Collision|SetCollisionEnabled (Variables|Default|GetSwordCollision) "NoCollision"))))
        (:then_2
          (Transformation|SetWorldTransform (Variables|Default|GetSword) (Math|Transform|MakeTransform (Transformation|GetSocketLocation _mesh "weapon_sword_r") (Transformation|GetSocketRotation _mesh "weapon_sword_r")) false false))))))

(fn ConstructionScript)

(fn GetIsCombat
  (return (Variables|Default|GetIsCombatRange)))