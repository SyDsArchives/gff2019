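; Character Blueprint that provides enemy-search overlap detection and a punch attack hit area.
; EnemySearch begin and end overlaps are forwarded to OnTestOverlapBegin and OnTestOverlapEnd, whose logic is not in this graph.
; Every Tick moves the Punch component to the mesh's hand_r socket location and rotation, with a negative unit scale.
; Debug print and explosion-spawn nodes are disconnected and never run.
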(event OnComponentBeginOverlap(EnemySearch)
  (params (OverlappedComponent :type Primitive%20Component%20Object%20Reference) (OtherActor :type Actor%20Object%20Reference) (OtherComp :type Primitive%20Component%20Object%20Reference) (OtherBodyIndex :type Integer) (bFromSweep :type Boolean) (SweepResult :type Hit%20Result%20Structure%20%28by%20ref%29))
  (Class|MyCharacter|OnTestOverlapBegin OtherActor OtherComp OtherBodyIndex bFromSweep))

(event OnComponentEndOverlap(EnemySearch)
  (params (OverlappedComponent :type Primitive%20Component%20Object%20Reference) (OtherActor :type Actor%20Object%20Reference) (OtherComp :type Primitive%20Component%20Object%20Reference) (OtherBodyIndex :type Integer))
  (Class|MyCharacter|OnTestOverlapEnd OtherActor OtherComp OtherBodyIndex))

(event EventTick
  (params (DeltaSeconds :type Float%20%28single-precision%29))
  (bind _mesh (Variables|Character|GetMesh))
  ;[1 1 1] パンチ攻撃判定
  (Transformation|SetWorldTransform (Variables|Default|GetPunch) (Math|Transform|MakeTransform (Transformation|GetSocketLocation _mesh "hand_r") (Transformation|GetSocketRotation _mesh "hand_r") "-1.000000,-1.000000,-1.000000") false false))

(fn ConstructionScript)